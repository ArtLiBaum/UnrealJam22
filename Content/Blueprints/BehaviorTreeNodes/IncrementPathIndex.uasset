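; Behavior tree task that advances an NPC's patrol path index to the next point.
; It reads the index from the blackboard and checks it against the PathPoints array on the controlled NPC's PatrolPath.
; It writes the incremented index and succeeds, or fails without wrapping when already at the last point.
; A failed cast to NPC stops execution without finishing the task.
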(event EventReceiveExecuteAI
  (params (OwnerController :type AI%20Controller%20Object%20Reference) (ControlledPawn :type Pawn%20Object%20Reference))
  (bind _bb_pathindex (Variables|Default|GetBB_PathIndex))
  (bind _returnvalue (Class|BTFunctionLibrary|GetBlackboardValueasInt _bb_pathindex))
  (bind _returnvalue_2 (+ _returnvalue 1))
  (bind _asnpc (Utilities|Casting|CastToNPC ControlledPawn))
  (if (<= _returnvalue_2 (- (Utilities|Array|Length (Variables|/Game/Blueprints/AI/NPC/PatrolPath.PatrolPath_C|GetPathPoints (Variables|/Game/Blueprints/AI/NPC/NPC.NPC_C|GetPatrolPath _asnpc))) 1))
    (Class|BTFunctionLibrary|SetBlackboardValueasInt (Variables|Default|GetBB_PathIndex) _returnvalue_2)
    (AI|BehaviorTree|FinishExecute true)
    (else
      (AI|BehaviorTree|FinishExecute false))))