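; Vacuum receptacle for animals that pulls in nearby suckable objects and rejects those of the wrong animal type.
; Overlap switches an idle object's TestSuckableComp state and sets its velocity from the suction point and speed; leaving range resets the state.
; A Box hit compares animal types and switches mismatches to a blow-back state.
; The step that teleports objects to the pen's deposit point is disconnected, so matches get no handling here.
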(event Collision|EventHit
  (params (MyComp :type Primitive%20Component%20Object%20Reference) (Other :type Actor%20Object%20Reference) (OtherComp :type Primitive%20Component%20Object%20Reference) (bSelfMoved :type Boolean) (HitLocation :type Vector :default "0, 0, 0") (HitNormal :type Vector :default "0, 0, 0") (NormalImpulse :type Vector :default "0, 0, 0") (Hit :type Hit%20Result%20Structure%20%28by%20ref%29))
  (bind _returnvalue (Actor|GetComponentbyClass Other "/Game/Blueprints/TestBps/TestSuckableComp.TestSuckableComp_C"))
  (bind _myanimaltype (Variables|Default|GetmyAnimalType))
  ;[1 1 1] ObjectHitsReceptacle
  ;;[1 1 1] If the object is colliding with the end of the vacuum and it is the right animal type
  (if (== MyComp (Variables|Default|GetBox))
    (Development|PrintString (Utilities|String|ToString(Byte) _myanimaltype))
    (if (not (Utilities|Enum|Equal(Enum) (Variables|/Game/Blueprints/TestBps/TestSuckableComp.TestSuckableComp_C|GetmyAnimalType _returnvalue) _myanimaltype))
      ;;[1 1 1] else, blow the object backwards
      (Variables|/Game/Blueprints/TestBps/TestSuckableComp.TestSuckableComp_C|SetmySuckState _returnvalue "NewEnumerator2"))))

(event Collision|EventActorBeginOverlap
  (params (OtherActor :type Actor%20Object%20Reference))
  (bind _returnvalue (Actor|GetComponentbyClass OtherActor "/Game/Blueprints/TestBps/TestSuckableComp.TestSuckableComp_C"))
  ;[1 1 1] When an object gets close enough to the vacuum, suck it in
  (if (Utilities|Enum|Equal(Enum) (Variables|/Game/Blueprints/TestBps/TestSuckableComp.TestSuckableComp_C|GetmySuckState _returnvalue) "NewEnumerator0")
    (Variables|/Game/Blueprints/TestBps/TestSuckableComp.TestSuckableComp_C|SetmySuckState _returnvalue "NewEnumerator1")
    (Variables|/Game/Blueprints/TestBps/TestSuckableComp.TestSuckableComp_C|SetSuckVel _returnvalue (* (Math|Vector|Normalize (- (Transformation|GetActorLocation OtherActor) (Variables|Default|GetSuctionPoint))) (Variables|Default|GetSuctionSpeed)))))

(event Collision|EventActorEndOverlap
  (params (OtherActor :type Actor%20Object%20Reference))
  ;[1 1 1] When an object leaves the range of the vacuum, stop affecting it
  (Variables|/Game/Blueprints/TestBps/TestSuckableComp.TestSuckableComp_C|SetmySuckState (Actor|GetComponentbyClass OtherActor "/Game/Blueprints/TestBps/TestSuckableComp.TestSuckableComp_C") "NewEnumerator0"))

(fn ConstructionScript)